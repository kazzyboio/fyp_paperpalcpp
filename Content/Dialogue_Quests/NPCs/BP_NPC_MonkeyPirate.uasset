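; Monkey pirate quest NPC that takes collected swords from the player, plays their insertion animations, and advances the castle and party quest dialogue.
; Talking inserts pending swords, sets StateIndex by progress, and plays level sequences before dialogue starts, with a separate final-sword sequence.
; Post-dialogue state updates accept quests, notify the TrashPaper NPC, show the guest-list popup, or open the alpha end screen.
; Certain states add a camera pan or hold back movement reactivation.
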(event `Play Animations`
  ;[1 1 1] Animations
  (if (`self.finalSword`)
    (set `self.finalSword` false)
    (`MovieSceneSequencePlayer.Play` (`LevelSequenceActor.SequencePlayer` (`self.lastSword`)))
    (set `self.playingAnimation` true)
    (`KismetSystemLibrary.Delay` 4.5)
    (elif (== (`self.totalInserted`) 3)
      (`MovieSceneSequencePlayer.Play` (`LevelSequenceActor.SequencePlayer` (`self.thirdSword`)))
      (if (not (`self.secondPlayed`))
        (`MovieSceneSequencePlayer.Play` (`LevelSequenceActor.SequencePlayer` (`self.secondSword`)) :!label _label)
        (set `self.secondPlayed` true)
        (if (not (`self.firstPlayed`))
          (`MovieSceneSequencePlayer.Play` (`LevelSequenceActor.SequencePlayer` (`self.firstSword`)) :!label _label_2)
          (set `self.firstPlayed` true)))
      (set `self.playingAnimation` true)
      (`KismetSystemLibrary.Delay` 1.5)
      (elif (== (`self.totalInserted`) 2)
        (goto _label)
        (elif (== (`self.totalInserted`) 1)
          (goto _label_2)
          (else
            _)))))
  (set `self.playingAnimation` false)
  (`self.Start Dialogue`))

(event `self.Pre Start Dialogue`
  ;[1 1 1] Insert Sword Check, Party Guests Count Check
  (if (not (`self.playingAnimation`))
    (if (`self.finalSword`)
      (`self.Insert Sword` :!label _label_3)
      (elif (> (`self.totalCollected`) 0)
        (goto _label_3)
        (else
          (`parent.Pre Start Dialogue`))))))

(event `Add Sword`
  ;[1 1 1] Add Sword
  (`/Engine/EditorBlueprintResources/StandardMacros.IncrementInt` (`self.totalCollected`)))

(event `Insert Sword`
  ;[1 1 1] Insert Sword
  (if (not (`self.finalSword`))
    (set `self.totalInserted` (+ (`self.totalInserted`) (`self.totalCollected`)))
    (set `self.totalCollected` 0)
    (if (== (`self.totalInserted`) (`self.totalNeeded`))
      (set `self.stateIndex` 4)
      (else
        (set `self.stateIndex` 3)))
    (else
      (set `self.stateIndex` 6)))
  (`self.Play Animations`))

(event `self.Post States Update`
  (bind _returnvalue (`GameplayStatics.GetPlayerController` 0))
  ;[1 1 1] Quest Update Changes
  (if (`self.castleQuestComplete`)
    (if (== (`self.stateIndex`) 1)
      (set `self.stateIndex` 2)
      (set `self.questAccepted` true)
      (elif (and (== (`self.stateIndex`) 3) (== (`self.totalCollected`) 0))
        (set `self.stateIndex` 2)
        (elif (== (`self.stateIndex`) 4)
          (set `self.stateIndex` 5)
          (bind _returnvalue_2 (`GameplayStatics.GetActorOfClass` "/Game/Dialogue_Quests/NPCs/BP_NPC_TrashPaper.BP_NPC_TrashPaper_C"))
          (`/Game/Dialogue_Quests/NPCs/BP_NPC_TrashPaper.Quest Accept Change` _returnvalue_2)
          (elif (== (`self.stateIndex`) 6)
            (set `self.stateIndex` 7)
            (set `self.partyQuestAccepted` true)
            ;[1 1 1] Guest List Popup
            (set `self.dialogueStart` true)
            (bind _returnvalue_3 (`GameplayStatics.GetActorOfClass` "/Game/PlayerCharacter/BP_Player.BP_Player_C"))
            (set `/Game/PlayerCharacter/BP_Player.inDialogue` true _returnvalue_3)
            (bind _returnvalue_4 (`|CreateWidget` "/Game/Assets/UI/WB/WB_GLPLACEHOLDER.WB_GLPLACEHOLDER_C" (`GameplayStatics.GetPlayerController` 0)))
            (`UserWidget.AddToViewport` _returnvalue_4 0)
            (`/Game/Assets/UI/WB/WB_GLPLACEHOLDER.Spawn Animation` _returnvalue_4)
            (set `self.dialogueStart` false)
            (elif (== (`self.stateIndex`) 8)
              (bind _returnvalue_5 (`|CreateWidget` "/Game/Assets/UI/WB/WB_EndScreenforAlpha.WB_EndScreenforAlpha_C" _returnvalue))
              (`UserWidget.AddToViewport` _returnvalue_5 0)
              (`WidgetBlueprintLibrary.SetInputMode_UIOnlyEx` _returnvalue null)
              (set `PlayerController.bShowMouseCursor` true _returnvalue))))))))

(event `self.Reactivate Movement`
  ;[1 1 1] Quest Update Changes
  (if (!= (`self.stateIndex`) 6)
    (`parent.Reactivate Movement`)))

(event `self.Camera Pan`
  (bind _blendtime (`self.blendTime`))
  (bind _stateindex (`self.stateIndex`))
  ;[1 1 1] Camera Pan
  (if (or (== _stateindex 4) (== _stateindex 5))
    (`PlayerController.SetViewTargetWithBlend` (`GameplayStatics.GetPlayerController` 0) (`self.cameraActor`) _blendtime "VTBlend_Linear" 0.0 false)
    (`KismetSystemLibrary.Delay` (+ _blendtime (`self.cameraStayTime`))))
  (`parent.Camera Pan`))

(fn `UserConstructionScript`
  (`parent.UserConstructionScript`))